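; Game state for a mosaic memory game that times the model-preview phase and the play round.
; BeginPlay starts the preview and fires a start event; Tick counts both timers down.
; When the preview ends it hides the player controller's grid colours, waits briefly and starts the round.
; When the round ends it awards points through the first player controller and broadcasts the score.
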(event EventBeginPlay
  (Variables|Default|SetShowModelMosaic true)
  (Default|CallOnModelMosaicStarted))

(event EventTick
  (params (DeltaSeconds :type Float%20%28single-precision%29))
  (Utilities|FlowControl|Sequence
    (:then_0
      (if (Variables|Default|GetShowModelMosaic)
        (if (<= (Variables|Default|GetModelMosaicTime) 0.0)
          (Variables|Default|SetShowModelMosaic false)
          (bind _asbp_mosaic_player_controller (Utilities|Casting|CastToBP_MosaicPlayerController (Game|GetPlayerController 0)))
          (Utilities|IsValid _asbp_mosaic_player_controller
            (:Is%20Valid
              (Default|HideColours (Variables|/Game/PlayerController/BP_MosaicPlayerController.BP_MosaicPlayerController_C|GetGridGenerator _asbp_mosaic_player_controller))
              (Utilities|FlowControl|Delay 1.5)
              (Variables|Default|SetShowNormalRoundTime true)
              (Default|CallOnRoundStarted)))
          (else
            (Variables|Default|SetModelMosaicTime (- (Variables|Default|GetModelMosaicTime) DeltaSeconds))))))
    (:then_1
      (if (Variables|Default|GetShowNormalRoundTime)
        (if (<= (Variables|Default|GetRoundTime) 0.0)
          (Variables|Default|SetShowNormalRoundTime false)
          (bind _asbp_mosaic_player_controller_2 (Utilities|Casting|CastToBP_MosaicPlayerController (Game|GetPlayerController 0)))
          (Utilities|IsValid _asbp_mosaic_player_controller_2
            (:Is%20Valid
              (Default|AddPoints _asbp_mosaic_player_controller_2)
              (Default|CallOnPointsAdded (Variables|/Game/PlayerController/BP_MosaicPlayerController.BP_MosaicPlayerController_C|GetPlayerScore _asbp_mosaic_player_controller_2))))
          (else
            (Variables|Default|SetRoundTime (- (Variables|Default|GetRoundTime) DeltaSeconds))))))))

(fn ConstructionScript)