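; Player controller for the Mosaic lobby that shows the lobby menu to the local player and can trigger server travel through the game instance.
; On BeginPlay it runs a server/client-named event chain that copies the start time and can-start flag from the lobby game state, then creates the menu widget.
; It also binds to the game state's lobby-started event, which only prints a debug message.
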(event Custom|LobbyStarted
  (Development|PrintString "LOBBY STARTED!"))

(event Custom|SetCanStartGameOnClient
  (CallFunction|TakeCanStartGamefromServer))

(event Custom|ClientStartGame
  (bind _asbp_mosaic_server_game_instance (Utilities|Casting|CastToBP_MosaicServerGameInstance (Game|GetGameInstance)))
  (Utilities|IsValid _asbp_mosaic_server_game_instance
    (:Is%20Valid
      (Default|TravelServer _asbp_mosaic_server_game_instance))))

(event Custom|SetTimerOnClient
  (CallFunction|TakeTimerValuefromServer))

(event Custom|TakeTimerValueFromServer
  (bind _asbp_mosaic_lobby_game_state (Utilities|Casting|CastToBP_MosaicLobbyGameState (Game|GetGameState)))
  (Variables|Default|SetLobbyTime (Variables|/Game/GameState/BP_MosaicLobbyGameState.BP_MosaicLobbyGameState_C|GetStartGameTime _asbp_mosaic_lobby_game_state)))

(event Custom|ShowLobbyWidgetOnServer
  (CallFunction|ShowLobbyWidgetonClient))

(event Custom|ShowLobbyWidgetOnClient
  (CallFunction|SetCanStartGameonClient)
  (CallFunction|SetTimeronClient)
  (if (Pawn|IsLocalPlayerController)
    (bind _returnvalue (UserInterface|CreateWidget "/Game/UI/WBP_MosaicLobbyMenu.WBP_MosaicLobbyMenu_C" (Game|GetPlayerController 0)))
    (Utilities|IsValid _returnvalue
      (:Is%20Valid
        (Variables|Default|SetLobbyMenuWidget _returnvalue)
        (UserInterface|Viewport|AddtoViewport _returnvalue 0)))))

(event Custom|TakeCanStartGameFromServer
  (bind _asbp_mosaic_lobby_game_state (Utilities|Casting|CastToBP_MosaicLobbyGameState (Game|GetGameState)))
  (Variables|Default|SetCanStartGame (Variables|/Game/GameState/BP_MosaicLobbyGameState.BP_MosaicLobbyGameState_C|GetCanStartGame _asbp_mosaic_lobby_game_state)))

(event EventBeginPlay
  (CallFunction|ShowLobbyWidgetonServer)
  (bind _asbp_mosaic_lobby_game_state (Utilities|Casting|CastToBP_MosaicLobbyGameState (Game|GetGameState)))
  (Utilities|IsValid _asbp_mosaic_lobby_game_state
    (:Is%20Valid
      (EventDispatchers|BindEventtoOnLobbyStarted _asbp_mosaic_lobby_game_state (delegate Custom|LobbyStarted)))))

(fn ConstructionScript)