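; Player controller for the Mosaic main menu that shows the menu UI and forwards session requests.
; On BeginPlay it creates the main menu widget, adds it to the viewport, switches to UI-only input and shows the mouse cursor.
; ClientHostSession and ClientJoinSession events cast the game instance to BP_MosaicServerGameInstance and call its HostSession or JoinSession.
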(event Custom|ClientHostSession
  (bind _asbp_mosaic_server_game_instance (Utilities|Casting|CastToBP_MosaicServerGameInstance (Game|GetGameInstance)))
  (Utilities|IsValid _asbp_mosaic_server_game_instance
    (:Is%20Valid
      (Default|HostSession _asbp_mosaic_server_game_instance))))

(event Custom|ClientJoinSession
  (bind _asbp_mosaic_server_game_instance (Utilities|Casting|CastToBP_MosaicServerGameInstance (Game|GetGameInstance)))
  (Utilities|IsValid _asbp_mosaic_server_game_instance
    (:Is%20Valid
      (Default|JoinSession _asbp_mosaic_server_game_instance))))

(event EventBeginPlay
  (bind _returnvalue (Game|GetPlayerController 0))
  (bind _returnvalue_2 (UserInterface|CreateWidget "/Game/UI/WBP_MosaicMainMenu.WBP_MosaicMainMenu_C" (Game|GetPlayerController 0)))
  (Utilities|IsValid _returnvalue_2
    (:Is%20Valid
      (UserInterface|Viewport|AddtoViewport _returnvalue_2 0)
      (Input|SetInputModeUIOnly _returnvalue _returnvalue_2 "DoNotLock")
      (Variables|/Script/Engine.PlayerController|SetbShowMouseCursor _returnvalue true))))

(fn ConstructionScript)