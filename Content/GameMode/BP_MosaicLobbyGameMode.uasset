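; Lobby game mode for Mosaic that counts down to the start of the game.
; BeginPlay broadcasts lobby start, then Tick drains StartGameTime and, at zero, sets CanStartGame and calls ClientStartGame on the first player controller only.
; A separate event asks the first player's character to show the lobby widget through the server, while other widget-display paths are left disconnected.
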(event Custom|StartGame
  (bind _asbp_mosaic_lobby_player_controller (Utilities|Casting|CastToBP_MosaicLobbyPlayerController (Game|GetPlayerController 0)))
  (Utilities|IsValid _asbp_mosaic_lobby_player_controller
    (:Is%20Valid
      (Default|ClientStartGame _asbp_mosaic_lobby_player_controller))))

(event Custom|ShowLobbyMenuWidget
  (bind _asthird_person_character (Utilities|Casting|CastToThirdPersonCharacter (Game|GetPlayerCharacter 0)))
  (Default|ShowLobbyWidgetonServer _asthird_person_character))

(event EventBeginPlay
  (Variables|Default|SetCanStartGame false)
  (Default|CallOnLobbyStarted))

(event EventTick
  (params (DeltaSeconds :type Float%20%28single-precision%29))
  (if (not (Variables|Default|GetCanStartGame))
    (if (<= (Variables|Default|GetStartGameTime) 0.0)
      (Variables|Default|SetCanStartGame true)
      (CallFunction|StartGame)
      (else
        (Variables|Default|SetStartGameTime (- (Variables|Default|GetStartGameTime) DeltaSeconds))))))

(fn ConstructionScript)