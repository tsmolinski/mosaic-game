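; BP_MosaicGridSection is one cell of a mosaic grid that places itself relative to its owning actor.
; InitSections attaches it to a valid owner, then sets its relative location from Column along Y and Row along Z, with a fixed 90-degree rotation.
; Spacing combines SectionsOffset with GridSection's bounds extents scaled by PivotSectionOffset, using the X extent for vertical spacing.
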(event EventBeginPlay)

(event Collision|EventActorBeginOverlap
  (params (OtherActor :type Actor%20Object%20Reference)))

(event EventTick
  (params (DeltaSeconds :type Float%20%28single-precision%29)))

(fn ConstructionScript)

(fn InitSections
  (bind _returnvalue (Components|GetOwner))
  (bind _row (Variables|Default|GetRow))
  (bind _column (Variables|Default|GetColumn))
  (bind _gridsection (Variables|Default|GetGridSection))
  (bind _boxextent (Collision|GetComponentBounds _gridsection))
  (bind (_x _y) (Math|Vector|BreakVector _boxextent))
  (Utilities|IsValid _returnvalue
    (:Is%20Valid
      (Transformation|AttachActorToActor _returnvalue "None" "SnapToTarget" "SnapToTarget" "KeepRelative" false)
      (Transformation|SetActorRelativeLocation (Math|Vector|MakeVector 0.0 (+ (* (Variables|Default|GetPivotSectionOffset) (* _column _y)) (Math|Conversions|ToFloat(Integer) (* _column (Variables|Default|GetSectionsOffset)))) (+ (Math|Conversions|ToFloat(Integer) (* (Variables|Default|GetSectionsOffset) _row)) (* (Variables|Default|GetPivotSectionOffset) (* _row _x)))))
      (Transformation|SetActorRelativeRotation "90.000000, 0, 0"))))