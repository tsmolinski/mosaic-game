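; BP_InteractionAreaCustomShape is an interaction area actor whose shape comes from a configurable static mesh.
; Its construction script applies CustomShape to the StaticMesh component, then either paints every material slot with M_InteractionShapeTrace when DevView is on or hides the mesh.
; It then runs the parent construction script; the event graph holds only disabled placeholder events.
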(event EventBeginPlay)

(event Collision|EventActorBeginOverlap
  (params (OtherActor :type Actor%20Object%20Reference)))

(event EventTick
  (params (DeltaSeconds :type Float%20%28single-precision%29)))

(fn ConstructionScript
  (Components|StaticMesh|SetStaticMesh (Variables|Default|GetStaticMesh) (Variables|Default|GetCustomShape))
  (if (Variables|Default|GetDevView)
    (for _array_element (Class|MeshComponent|GetMaterialSlotNames (Variables|Default|GetStaticMesh))
      (Rendering|Material|SetMaterialbyName (Variables|Default|GetStaticMesh) _array_element "/Game/Materials/M_InteractionShapeTrace.M_InteractionShapeTrace"))
    (else
      (Rendering|SetVisibility (Variables|Default|GetStaticMesh) false false)))
  (|CallParentFunction))