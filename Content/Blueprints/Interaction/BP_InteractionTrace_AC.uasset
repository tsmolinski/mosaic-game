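; Interaction component that finds the interaction area the player looks at and triggers it.
; Each Tick a Visibility line trace runs from the follow camera, starting past the boom length, and switches focus between box and custom-shape areas.
; TryToInteract fires immediately or starts a countdown from the area's duration, which focus changes cancel, with started and disrupted dispatchers.
; InteractOnServer then sends InteractMessage to the area's parent actor.
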(event Custom|TryToInteract
  (params (In :type Boolean))
  (if In
    (if (Variables|Default|GetTracingInteractionArea)
      (bind _output_get (Variables|Default|SetInteraction%20Duration (Variables|/Game/Blueprints/Interaction/BP_InteractionAreaMaster.BP_InteractionAreaMaster_C|GetInteractionDuration (Variables|Default|GetFocusedInteractionArea))))
      (if (> _output_get 0.0)
        (Variables|Default|SetTempDuration (Variables|Default|GetInteraction%20Duration))
        (Default|CallOnInteractionStarted)
        (Variables|Default|SetIsInteracting true)
        (else
          (CallFunction|InteractonServer (Variables|Default|GetFocusedInteractionArea)))))))

(event Custom|InteractOnServer
  (params (InteractionArea :type BP%20Interaction%20Area%20Master%20Object%20Reference))
  (Class|BPIInteraction|Interact(Message) (Actor|GetParentActor InteractionArea)))

(event EventTick
  (params (DeltaSeconds :type Float%20%28single-precision%29))
  (CallFunction|Trace)
  (if (Variables|Default|GetIsInteracting)
    (bind _output_get (Variables|Default|SetTempDuration (- (Variables|Default|GetTempDuration) DeltaSeconds)))
    (if (<= _output_get 0.0)
      (Variables|Default|SetIsInteracting false)
      (CallFunction|InteractonServer (Variables|Default|GetFocusedInteractionArea)))))

(fn TraceInteractionArea
  (params (Trace :type Boolean))
  (if Trace
    (if (Variables|Default|GetTracingInteractionArea)
      (Utilities|FlowControl|Sequence
        (:then_0
          ;[1 1 1] Disable focus on "old" int area
          (Default|SetFocus (Variables|Default|GetFocusedInteractionArea) false)
          (Variables|Default|SetIsInteracting false)
          (Default|CallOnInteractionDisrupted))
        (:then_1
          (bind _asbp_interaction_area_master (Utilities|Casting|CastToBP_InteractionAreaMaster (Variables|Default|GetFocusedActor)))
          (bind _output_get (Variables|Default|SetFocusedInteractionArea _asbp_interaction_area_master))
          (Default|SetFocus _output_get true)
          (Variables|Default|SetTracingInteractionArea true)))
      (else
        (bind _asbp_interaction_area_master_2 (Utilities|Casting|CastToBP_InteractionAreaMaster (Variables|Default|GetFocusedActor)))
        (bind _output_get_2 (Variables|Default|SetFocusedInteractionArea _asbp_interaction_area_master_2))
        (Default|SetFocus _output_get_2 true)
        (Variables|Default|SetTracingInteractionArea true)))
    (elif (Variables|Default|GetTracingInteractionArea)
      (Variables|Default|SetTracingInteractionArea false)
      (Variables|Default|SetIsInteracting false)
      (Default|SetFocus (Variables|Default|GetFocusedInteractionArea) false)
      (Variables|Default|SetFocusedActor 0)
      (Variables|Default|SetFocusedInteractionArea 0)
      (Default|CallOnInteractionDisrupted))))

(fn Trace
  (bind _asthird_person_character (Utilities|Casting|CastToThirdPersonCharacter (Game|GetPlayerCharacter 0)))
  (bind (_outhit _returnvalue) (Collision|LineTraceByChannel (+ (Transformation|GetWorldLocation (Variables|/Game/Character/ThirdPersonCharacter.ThirdPersonCharacter_C|GetFollowCamera _asthird_person_character)) (* (Math|Vector|GetForwardVector (Variables|/Game/Character/ThirdPersonCharacter.ThirdPersonCharacter_C|GetFollowCamera _asthird_person_character)) (Variables|/Script/Engine.SpringArmComponent|GetTargetArmLength (Variables|/Game/Character/ThirdPersonCharacter.ThirdPersonCharacter_C|GetCameraBoom _asthird_person_character)))) (+ (Transformation|GetWorldLocation (Variables|/Game/Character/ThirdPersonCharacter.ThirdPersonCharacter_C|GetFollowCamera _asthird_person_character)) (* (Math|Vector|GetForwardVector (Variables|/Game/Character/ThirdPersonCharacter.ThirdPersonCharacter_C|GetFollowCamera _asthird_person_character)) (Variables|Default|GetLength))) "TraceTypeQuery1" false 0 "ForDuration"))
  (if _returnvalue
    (if (!= (Variables|Default|GetFocusedActor) (.HitActor (Collision|BreakHitResult _outhit)))
      (Variables|Default|SetFocusedActor (.HitActor (Collision|BreakHitResult _outhit)))
      (CallFunction|TraceInteractionArea (or (== (Utilities|GetClass (.HitActor (Collision|BreakHitResult _outhit))) "/Game/Blueprints/Interaction/BP_InteractionAreaBox.BP_InteractionAreaBox_C") (== (Utilities|GetClass (.HitActor (Collision|BreakHitResult _outhit))) "/Game/Blueprints/Interaction/BP_InteractionAreaCustomShape.BP_InteractionAreaCustomShape_C"))))
    (else
      ;[1 1 1] Is it neccessary?
      (CallFunction|TraceInteractionArea false))))