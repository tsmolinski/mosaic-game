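; BP_ColourBucket is a bucket actor that attaches to its owner and positions itself in a row by its bucket number.
; InitBuckets, when the owner is valid, attaches the bucket with location and rotation snapped, then calls SetLocation.
; SetLocation spaces it along the relative Y axis, multiplying the bucket number by the Cube's bounds extent scaled by a pivot offset, plus a per-bucket gap.
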(event EventBeginPlay)

(event Collision|EventActorBeginOverlap
  (params (OtherActor :type Actor%20Object%20Reference)))

(event EventTick
  (params (DeltaSeconds :type Float%20%28single-precision%29)))

(fn ConstructionScript)

(fn InitBuckets
  (bind _returnvalue (Components|GetOwner))
  (Utilities|IsValid _returnvalue
    (:Is%20Valid
      (Transformation|AttachActorToActor _returnvalue "None" "SnapToTarget" "SnapToTarget" "KeepRelative" false)
      (CallFunction|SetLocation))))

(fn SetLocation
  (bind _sweephitresult (Transformation|SetActorRelativeLocation (Math|Vector|MakeVector 0.0 (+ (* (Variables|Default|GetPivotBucketOffset) (* (Variables|Default|GetBucketNumber) (.Y (Math|Vector|BreakVector (.BoxExtent (Collision|GetComponentBounds (Variables|Default|GetCube))))))) (Math|Conversions|ToFloat(Integer) (* (Variables|Default|GetBucketOffset) (Variables|Default|GetBucketNumber)))) 0.0)))
  (return _sweephitresult))