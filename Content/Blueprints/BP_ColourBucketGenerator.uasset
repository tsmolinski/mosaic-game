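; BP_ColourBucketGenerator spawns one colour bucket for each colour defined on the mosaic player controller.
; On BeginPlay, Init destroys any tracked buckets, then spawns each at the generator's transform with its array index as BucketNumber and calls InitBuckets.
; It tints each bucket's cube through the Colour material parameter and registers the bucket-to-colour pairing in the controller's BucketColourMap.
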(event EventBeginPlay
  (CallFunction|Init))

(event Collision|EventActorBeginOverlap
  (params (OtherActor :type Actor%20Object%20Reference)))

(event EventTick
  (params (DeltaSeconds :type Float%20%28single-precision%29)))

(fn ConstructionScript)

(fn Clear
  (bind _buckets (Variables|Default|GetBuckets))
  (if (> (Utilities|Array|Length (Variables|Default|GetBuckets)) 0)
    (for _array_element _buckets
      (Actor|DestroyActor _array_element))
    (Utilities|Array|Clear _buckets)))

(fn Init
  (CallFunction|Clear)
  (bind _asbp_mosaic_player_controller (Utilities|Casting|CastToBP_MosaicPlayerController (Game|GetPlayerController 0)))
  (for (_array_element _array_index) (Variables|/Game/PlayerController/BP_MosaicPlayerController.BP_MosaicPlayerController_C|GetColours _asbp_mosaic_player_controller)
    (bind _returnvalue (Game|SpawnActorfromClass "/Game/Blueprints/BP_ColourBucket.BP_ColourBucket_C" (Math|Transform|MakeTransform (Transformation|GetActorLocation) (Transformation|GetActorRotation)) "Undefined" self _array_index 0))
    (Default|InitBuckets _returnvalue)
    (Utilities|Array|Add (Variables|Default|GetBuckets) _returnvalue)
    (Rendering|Material|SetVectorParameterValueonMaterials (Variables|/Game/Blueprints/BP_ColourBucket.BP_ColourBucket_C|GetCube _returnvalue) "Colour" (Math|Conversions|ToVector(LinearColor) _array_element))
    (bind _asbp_mosaic_player_controller_2 (Utilities|Casting|CastToBP_MosaicPlayerController (Game|GetPlayerController 0)))
    (Utilities|Map|Add (Variables|/Game/PlayerController/BP_MosaicPlayerController.BP_MosaicPlayerController_C|GetBucketColourMap _asbp_mosaic_player_controller_2) _returnvalue _array_element)))