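; BP_MosaicGridGenerator is an actor that builds a mosaic grid of BP_MosaicGridSection actors when play begins.
; Init calls Clear to destroy any tracked sections, then loops over Rows and Columns to spawn one half-scale, owned section per cell.
; All sections spawn at the generator's location and rotation, receiving their Row and Column before InitSections runs and they are stored in Sections.
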(event EventBeginPlay
  (CallFunction|Init))

(event Collision|EventActorBeginOverlap
  (params (OtherActor :type Actor%20Object%20Reference)))

(event EventTick
  (params (DeltaSeconds :type Float%20%28single-precision%29)))

(fn ConstructionScript)

(fn Clear
  (bind _sections (Variables|Default|GetSections))
  (if (> (Utilities|Array|Length (Variables|Default|GetSections)) 0)
    (for _array_element _sections
      (Actor|DestroyActor _array_element))
    (Utilities|Array|Clear _sections)))

(fn Init
  (CallFunction|Clear)
  (for _index (range 0 (- (Variables|Default|GetRows) 1))
    (for _index_2 (range 0 (- (Variables|Default|GetColumns) 1))
      (bind _returnvalue (Game|SpawnActorfromClass "/Game/Blueprints/BP_MosaicGridSection.BP_MosaicGridSection_C" (Math|Transform|MakeTransform (Transformation|GetActorLocation) (Transformation|GetActorRotation) "0.500000,0.500000,0.500000") "AlwaysSpawn" self _index _index_2 0))
      (Default|InitSections _returnvalue)
      (Utilities|Array|Add (Variables|Default|GetSections) _returnvalue))))