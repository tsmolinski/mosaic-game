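; Game instance Blueprint that handles online session hosting, joining and server travel for multiplayer play.
; HostSession creates a four-connection non-LAN session and, on success, opens the lobby map as a listen server.
; JoinSession finds non-LAN sessions, loops over the results with an empty body, then joins using the loop's array element.
; TravelServer moves the server to the game map through a servertravel console command.
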(event Custom|JoinSession
  (bind _results (|FindSessions (Game|GetPlayerController 0) 0 false)
    (:OnSuccess
      (for _array_element _results
        _)
      (|JoinSession (Game|GetPlayerController 0) _array_element))))

(event Custom|HostSession
  (|Session (Game|GetPlayerController 0) 4 false
    (:OnSuccess
      (Game|OpenLevel(byObjectReference) (Variables|Default|GetLobbyMap) true "Listen"))))

(event Custom|TravelServer
  (Development|ExecuteConsoleCommand (Utilities|String|Append "servertravel " (Variables|Default|GetGameMapName)) 0))