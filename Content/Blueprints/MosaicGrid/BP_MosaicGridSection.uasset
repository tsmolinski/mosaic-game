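; BP_MosaicGridSection is a single section actor of a mosaic grid that places itself relative to its owning actor by row and column.
; InitSections snaps it to a valid owner, calls SetLocation, then applies a fixed 90-degree relative rotation.
; SetLocation spaces it along Y by column and Z by row, using GridSection bounds, a pivot multiplier and a gap offset.
; BeginPlay and the construction script are empty.
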(event EventBeginPlay)

(fn ConstructionScript)

(fn InitSections
  (bind _returnvalue (Components|GetOwner))
  (Utilities|IsValid _returnvalue
    (:Is%20Valid
      (Transformation|AttachActorToActor _returnvalue "None" "SnapToTarget" "SnapToTarget" "KeepRelative" false)
      (CallFunction|SetLocation)
      (Transformation|SetActorRelativeRotation "90.000000, 0, 0"))))

(fn SetLocation
  (bind _row (Variables|Default|GetRow))
  (bind _column (Variables|Default|GetColumn))
  (bind _gridsection (Variables|Default|GetGridSection))
  (bind _boxextent (Collision|GetComponentBounds _gridsection))
  (bind (_x _y) (Math|Vector|BreakVector _boxextent))
  (bind _sweephitresult (Transformation|SetActorRelativeLocation (Math|Vector|MakeVector 0.0 (+ (* (Variables|Default|GetPivotSectionOffset) (* _column _y)) (Math|Conversions|ToFloat(Integer) (* _column (Variables|Default|GetSectionsOffset)))) (+ (Math|Conversions|ToFloat(Integer) (* (Variables|Default|GetSectionsOffset) _row)) (* (Variables|Default|GetPivotSectionOffset) (* _row _x))))))
  (return _sweephitresult))