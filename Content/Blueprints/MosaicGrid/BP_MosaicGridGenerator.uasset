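; Grid generator actor that spawns the mosaic's BP_MosaicGridSection actors on BeginPlay.
; BeginPlay chains InitOnServer and InitOnClient into Init, which loops over Rows and Columns, spawning half-scale sections at its own transform with their indices and calling InitSections on each.
; Each section registers in player controller 0's MosaicSections.
; Clear, HideColours and AddRandomColours are empty, their clearing and colouring logic left disconnected.
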(event Custom|InitOnClient
  (CallFunction|Init))

(event Custom|InitOnServer
  (CallFunction|InitonClient))

(event EventBeginPlay
  (CallFunction|InitonServer))

(fn ConstructionScript)

(fn Clear)

(fn Init
  (CallFunction|Clear)
  (for _index (range 0 (- (Variables|Default|GetRows) 1))
    (for _index_2 (range 0 (- (Variables|Default|GetColumns) 1))
      (bind _returnvalue (Game|SpawnActorfromClass "/Game/Blueprints/MosaicGrid/BP_MosaicGridSection.BP_MosaicGridSection_C" (Math|Transform|MakeTransform (Transformation|GetActorLocation) (Transformation|GetActorRotation) "0.500000,0.500000,0.500000") "AlwaysSpawn" self _index _index_2 0))
      (Default|InitSections _returnvalue)
      (bind _asbp_mosaic_player_controller (Utilities|Casting|CastToBP_MosaicPlayerController (Game|GetPlayerController 0)))
      (Utilities|Set|Add (Variables|/Game/PlayerController/BP_MosaicPlayerController.BP_MosaicPlayerController_C|GetMosaicSections _asbp_mosaic_player_controller) _returnvalue))))

(fn HideColours)

(fn AddRandomColours)